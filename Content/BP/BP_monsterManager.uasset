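; Manager for a survive-until-6-AM night game that drives a left/right monster threat, the clock, and win and game-over screens.
; A looping timer either retreats a revealed monster or rolls against Difficulty to teleport a hidden one to either side.
; Tick advances hours toward the win and checks player distance to both monsters, playing one-shot sounds.
; Proximity feeds a shared countdown to game over, reset when both are out of range.
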(event Custom|CheckMonsterMove
  (if (Variables|Default|GetIsMonsterRevealed)
    (CallFunction|MonsterRetreat)
    (Variables|Default|SetIsMonsterRevealed false)
    (elif (<= (Variables|Default|GetDifficulty) (Math|Random|RandomIntegerinRange 0 100))
      (switch int (Variables|Default|GetMonsterLocation)
        (:0
          (Variables|Default|SetMonsterLocation (Math|Random|RandomIntegerinRange 1 2))
          (CallFunction|UpdateMonsterVisual))))))

(event Custom|UpdateMonsterVisual
  (switch int (Variables|Default|GetMonsterLocation)
    (:0
      (Transformation|SetActorLocation (Variables|Default|GetMonsterLeft_Ref) "999.000000,99.000000,999.000000" false false)
      (Transformation|SetActorLocation (Variables|Default|GetMonsterRight_Ref) "999.000000,99.000000,999.000000" false false))
    (:1
      (Transformation|SetActorLocation (Variables|Default|GetMonsterLeft_Ref) "344.000000,148.000000,72.000000" false false))
    (:2
      (Transformation|SetActorLocation (Variables|Default|GetMonsterRight_Ref) "-453.000000,148.000000,72.000000" false false))))

(event Custom|MonsterRetreat
  (Variables|Default|SetMonsterLocation 0)
  (CallFunction|UpdateMonsterVisual)
  (Development|PrintString "I got the signal from Player!")
  (Variables|Default|SetIsMonsterRevealed false))

(event Custom|UpdateGameTime
  (bind _output_get (Variables|Default|SetTargetTime 1.0))
  (if (<= _output_get 0.0)
    (Development|PrintString "6 AM")))

(event EventBeginPlay
  (Utilities|Time|SetTimerbyEvent (delegate Custom|CheckMonsterMove) 8.0 true))

(event Collision|EventActorBeginOverlap
  (params (OtherActor :type Actor%20Object%20Reference)))

(event EventTick
  (params (DeltaSeconds :type Float%20%28single-precision%29))
  (bind _returnvalue (Game|GetPlayerController 0))
  (bind _returnvalue_2 (Game|GetPlayerController 0))
  (Utilities|FlowControl|Sequence
    (:then_0
      (Variables|Default|SetGameMinutes (+ (Variables|Default|GetGameMinutes) (Utilities|Time|GetWorldDeltaSeconds)))
      (if (>= (Variables|Default|GetGameMinutes) 4e+01)
        (Variables|Default|SetCurrentHour (+ (Variables|Default|GetCurrentHour) 1))
        (Variables|Default|SetGameMinutes 0.0)
        (if (>= (Variables|Default|GetCurrentHour) 6)
          (Game|SetGamePaused true)
          (bind _returnvalue_3 (UserInterface|CreateWidget "/Game/WBP_WinScreen.WBP_WinScreen_C"))
          (UserInterface|Viewport|AddtoViewport _returnvalue_3 0)
          (Input|SetInputModeUIOnly _returnvalue 0 "DoNotLock" false)
          (Variables|/Script/Engine.PlayerController|SetbShowMouseCursor _returnvalue true))))
    (:then_1
      (bind _monsterleft_ref (Variables|Default|GetMonsterLeft_Ref)
        (:then
          (if (<= (Transformation|GetDistanceTo (Game|GetPlayerCharacter 0) _monsterleft_ref) 1e+03)
            (Utilities|FlowControl|Sequence
              (:then_0
                (Variables|Default|Set1 false)
                (Variables|Default|SetStartTimer (+ (Variables|Default|GetStartTimer) (Utilities|Time|GetWorldDeltaSeconds)) :!label _label)
                (if (>= (Variables|Default|GetStartTimer) 5.0)
                  (bind _returnvalue_4 (UserInterface|CreateWidget "/Game/WBP_GameOver.WBP_GameOver_C"))
                  (UserInterface|Viewport|AddtoViewport _returnvalue_4 0)
                  (Input|SetInputModeUIOnly _returnvalue_2 0 "DoNotLock" false)
                  (Variables|/Script/Engine.PlayerController|SetbShowMouseCursor _returnvalue_2 true)
                  (Game|SetGamePaused true)))
              (:then_1
                (Utilities|FlowControl|DoOnce false :!label _label_2
                  (:Completed
                    (Audio|PlaySoundatLocation "/Game/music/Hehehe_Cue.Hehehe_Cue" (Transformation|GetActorLocation (Variables|Default|GetMonsterLeft_Ref)) "0, 0, 0" 1.0 1.0 0.0 0 0 0 0)))))
            (else
              (Utilities|FlowControl|Sequence
                (:then_0
                  (bind _output_get (Variables|Default|Set1 true))
                  (if (and _output_get (stale _output_get_2)) :!label _label_3
                    (Variables|Default|SetStartTimer 0.0)))
                (:then_1
                  (goto _label_2 Reset))))))
        (:else)))
    (:then_2
      (bind _monsterright_ref (Variables|Default|GetMonsterRight_Ref)
        (:then
          (if (<= (Transformation|GetDistanceTo (Game|GetPlayerCharacter 0) _monsterright_ref) 1e+03)
            (Utilities|FlowControl|Sequence
              (:then_0
                (Variables|Default|Set2 false)
                (goto _label))
              (:then_1
                (Utilities|FlowControl|DoOnce false :!label _label_4
                  (:Completed
                    (Audio|PlaySoundatLocation "/Game/music/Hey_Cue.Hey_Cue" (Transformation|GetActorLocation (Variables|Default|GetMonsterRight_Ref)) "0, 0, 0" 1.0 1.0 0.0 0 0 0 0)))))
            (else
              (Utilities|FlowControl|Sequence
                (:then_0
                  (bind _output_get_2 (Variables|Default|Set2 true))
                  (goto _label_3))
                (:then_1
                  (goto _label_4 Reset))))))
        (:else)))))

(fn ConstructionScript)